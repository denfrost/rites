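; BP_Fighter is a fighter Blueprint that flags inventory and HUD widgets as out of date.
; Two events fetch the named menu from BP_RitesGameInstance and cast it to W_Inventory or W_HUD.
; They then set the inventory's Dirty flag or the HUD's HealthDirty flag.
; The default BeginPlay, overlap and Tick events and the construction script are empty.
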(event `self.DirtyInventoryMenu`
  (bind _asbp_rites_game_instance (cast `/Game/Blueprints/BP_RitesGameInstance` (`GameplayStatics.GetGameInstance`)))
  (bind _openedmenu (`/Game/Blueprints/BP_RitesGameInstance.GetMenu` _asbp_rites_game_instance "Inventory"))
  (bind _asw_inventory (cast `/Game/Widgets/Menus/W_Inventory` _openedmenu))
  (set `/Game/Widgets/Menus/W_Inventory.Dirty` true _asw_inventory))

(event `self.DirtyHUDMenu`
  (params (bDirtyHealth :type Boolean))
  (bind _asbp_rites_game_instance (cast `/Game/Blueprints/BP_RitesGameInstance` (`GameplayStatics.GetGameInstance`)))
  (bind _openedmenu (`/Game/Blueprints/BP_RitesGameInstance.GetMenu` _asbp_rites_game_instance "HUD"))
  (bind _asw_hud (cast `/Game/Widgets/HUD/W_HUD` _openedmenu))
  (set `/Game/Widgets/HUD/W_HUD.HealthDirty` true _asw_hud))

(fn `UserConstructionScript`)