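; BP_RitesGameInstance is a game instance that manages named UI menus, joins online sessions and provides a gem color lookup.
; OpenMenu creates a widget from a name-to-class map, adds it to the viewport and tracks it in an instance map, which CloseMenu and the query functions use.
; JoinRitesSession joins a given search result with the first player controller, and GetColorFromGemColor resolves gem colors through a map.
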(event `self.OpenMenu`
  (params (Name :type String))
  (bind (_value _returnvalue) (`BlueprintMapLibrary.Map_Find` (`self.MenuNameToClassMap`) Name))
  (if (not (`self.IsMenuOpen` Name))
    (if _returnvalue
      (bind _returnvalue_2 (`|CreateWidget` _value))
      (`UserWidget.AddToViewport` _returnvalue_2 0)
      (`BlueprintMapLibrary.Map_Add` (`self.MenuNameToInstanceMap`) Name _returnvalue_2))))

(event `self.CloseMenu`
  (params (Name :type String))
  (bind (_value _returnvalue) (`BlueprintMapLibrary.Map_Find` (`self.MenuNameToInstanceMap`) Name))
  (if (`self.IsMenuOpen` Name)
    (if _returnvalue
      (`Widget.RemoveFromParent` _value)
      (`BlueprintMapLibrary.Map_Remove` (`self.MenuNameToInstanceMap`) Name)
      (else
        (`KismetSystemLibrary.PrintString` "Failed to Remove Menu" true true (struct :`R` 1.0 :`G` 0.432646 :`A` 1.0))))))

(event `Join Rites Session`
  (params (SessionResult :type "BlueprintSessionResult Structure"))
  (`JoinSessionCallbackProxy.JoinSession` (`GameplayStatics.GetPlayerController` 0) SessionResult))

(fn `GetColorFromGemColor`
  (params (GemColor :type "EGemColor Enum" :default "Red"))
  (returns (ReturnValue :type "Color Structure"))
  (return (`BlueprintMapLibrary.Map_Find` (`self.GemColorToColorMap`) GemColor)))

(fn `GetMenu`
  (params (MenuName :type String))
  (returns (OpenedMenu :type "UserWidget Object Reference"))
  (return (`BlueprintMapLibrary.Map_Find` (`self.MenuNameToInstanceMap`) MenuName)))

(fn `IsMenuOpen`
  (params (Name :type String))
  (returns (ReturnValue :type Boolean))
  (return (`BlueprintMapLibrary.Map_Contains` (`self.MenuNameToInstanceMap`) Name)))