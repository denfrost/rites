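; BP_DDRMachine is a DDR machine prop whose two speakers hover up and down.
; BeginPlay caches the relative Z of Speaker1 as the shared rest height for both speakers.
; Tick accumulates a hover timer and offsets both speakers from that height by a sine wave scaled by an amplitude variable, so they bob in sync while keeping their own X and Y.
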(event `self.ReceiveBeginPlay`
  (bind (_relativelocation_x _relativelocation_y _relativelocation_z) (`KismetMathLibrary.BreakVector` (`SceneComponent.RelativeLocation` (`self.Speaker1`))))
  (set `self.InitialSpeakerZ` _relativelocation_z))

(event `self.ReceiveTick`
  (params (DeltaSeconds :type "Float (single-precision)"))
  (bind _speaker2 (`self.Speaker2`))
  (bind _speaker1 (`self.Speaker1`))
  (bind (_relativelocation_x _relativelocation_y) (`KismetMathLibrary.BreakVector` (`SceneComponent.RelativeLocation` _speaker1)))
  (bind (_relativelocation_x_2 _relativelocation_y_2) (`KismetMathLibrary.BreakVector` (`SceneComponent.RelativeLocation` _speaker2)))
  (bind _output_get (set `self.HoverTime` (+ DeltaSeconds (`self.HoverTime`))))
  (bind _returnvalue (+ (* (`KismetMathLibrary.Sin` _output_get) (`self.SpeakerHoverAmplitude`)) (`self.InitialSpeakerZ`)))
  (`SceneComponent.K2_SetRelativeLocation` _speaker1 (`KismetMathLibrary.MakeVector` _relativelocation_x _relativelocation_y _returnvalue) false false)
  (`SceneComponent.K2_SetRelativeLocation` _speaker2 (`KismetMathLibrary.MakeVector` _relativelocation_x_2 _relativelocation_y_2 _returnvalue) false false))

(fn `UserConstructionScript`)